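; BP_PainelSenha is an interactable password keypad that blends the view to itself and switches to UI-only input.
; ExecutarAcao starts interaction and immediately compares the stored entry to a hardcoded code, printing the result.
; While interacting, number keys feed Registrarnum, which appends and prints digits, clearing the entry at four characters.
; Q blends back to the player character, restores game input and ends interaction.
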(event `/Game/FirstPerson/Blueprints/BPI_Interacao.ExecutarAcao`
  (set `self.estouinteragindo` true)
  (`PlayerController.SetViewTargetWithBlend` (`GameplayStatics.GetPlayerController` 0) self 0.5 "VTBlend_Linear" 0.0 false)
  (`WidgetBlueprintLibrary.SetInputMode_UIOnlyEx` null null)
  (if (== (`self.senhadigitada`) 123)
    (`KismetSystemLibrary.PrintString` "senha correta" true true (struct :`G` 0.66 :`B` 1.0 :`A` 1.0) 5.0)
    (else
      (`KismetSystemLibrary.PrintString` "senha incorreta" true true (struct :`G` 0.66 :`B` 1.0 :`A` 1.0) 5.0))))

(event `Key|Q`
  (params (Key :type "Key Structure"))
  (:`Pressed`
    (`PlayerController.SetViewTargetWithBlend` (`GameplayStatics.GetPlayerController` 0) (`GameplayStatics.GetPlayerCharacter` 0) 0.5 "VTBlend_Linear" 0.0 false)
    (`WidgetBlueprintLibrary.SetInputMode_GameOnly` null)
    (set `self.estouinteragindo` false)))

(event `Key|Zero`
  (params (Key :type "Key Structure"))
  (:`Pressed`
    (`self.registrarnum` "0")))

(event `Key|Five`
  (params (Key :type "Key Structure"))
  (:`Pressed`
    (`self.registrarnum` "5")))

(event `Key|One`
  (params (Key :type "Key Structure"))
  (:`Pressed`
    (`self.registrarnum` "1")))

(event `Key|Six`
  (params (Key :type "Key Structure"))
  (:`Pressed`
    (`self.registrarnum` "6")))

(event `Key|Seven`
  (params (Key :type "Key Structure"))
  (:`Pressed`
    (`self.registrarnum` "7")))

(event `Key|Two`
  (params (Key :type "Key Structure"))
  (:`Pressed`
    (`self.registrarnum` "2")))

(event `Key|Eight`
  (params (Key :type "Key Structure"))
  (:`Pressed`
    (`self.registrarnum` "8")))

(event `Key|Three`
  (params (Key :type "Key Structure"))
  (:`Pressed`
    (`self.registrarnum` "3")))

(event `Key|Nine`
  (params (Key :type "Key Structure"))
  (:`Pressed`
    (`self.registrarnum` "9")))

(event `Key|Four`
  (params (Key :type "Key Structure"))
  (:`Pressed`
    (`self.registrarnum` "4")))

(fn `registrarnum`
  (params (numdigitado :type String))
  (bind _senhadigitada (`self.senhadigitada`))
  (if (`self.estouinteragindo`)
    (bind _output_get (set `self.senhadigitada` (`KismetStringLibrary.Concat_StrStr` _senhadigitada numdigitado)))
    (if (>= (`KismetStringLibrary.Len` _output_get) 4)
      (set `self.senhadigitada` "")
      (else
        (`KismetSystemLibrary.PrintString` _senhadigitada)))))

(fn `UserConstructionScript`)